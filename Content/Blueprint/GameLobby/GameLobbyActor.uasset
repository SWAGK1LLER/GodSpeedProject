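; GameLobbyActor represents a player in the game lobby with a skeletal mesh and a name widget.
; SetPlayerNameLocal relays the name through SetPlayerNameMult to SetPlayerName, which writes it into the UserNameWidget.
; A RepNotify on Mesh applies the skeletal mesh asset, and Disconnect marks the actor's GameLobbySpawn slot as unused.
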(event `SetPlayerNameMult`
  (params (name :type String))
  (`self.SetPlayerName` name))

(event `SetPlayerNameLocal`
  (params (name :type String))
  (`self.SetPlayerNameMult` name))

(fn `Disconnect`
  (set `/Game/Blueprint/GameLobby/GameLobbySpawn.SlotUsed` false (`self.GameLobbySpawn`)))

(fn `OnRep_mesh`
  (`SkeletalMeshComponent.SetSkeletalMeshAsset` (`self.SkeletalMesh`) (`self.mesh`)))

(fn `SetPlayerName`
  (params (name :type String))
  (bind _asuser_name_widget (cast `/Game/Blueprint/MainMenu/UserNameWidget` (`WidgetComponent.GetWidget` (`self.Widget`))))
  (`/Game/Blueprint/MainMenu/UserNameWidget.SetName` _asuser_name_widget (`KismetTextLibrary.Conv_StringToText` name)))

(fn `UserConstructionScript`)