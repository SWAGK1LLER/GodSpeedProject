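; Lobby game mode that places each player's display actor on a spawn slot and coordinates party state across player controllers.
; InitPlayer claims a free LobbySpawn, spawns a named LobbyActor there, and hides the quit-party button for a lone player or search for later joiners.
; Controllers gathered at PostLogin receive team changes and, when later players claim slots, slot occupancy updates.
; OnLogout only casts the controller, so neither slots nor the list are cleaned up.
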(event `SetTeam`
  (params (team :type "ETeam Enum" :default "A"))
  (for _array_element (`self.pcs`)
    (bind _aslobby_pc (cast `/Game/Blueprint/Lobby/LobbyPC` _array_element))
    (`/Game/Blueprint/Lobby/LobbyPC.SetTeam` _aslobby_pc team)))

(event `self.K2_PostLogin`
  (params (NewPlayer :type "PlayerController Object Reference"))
  (`KismetArrayLibrary.Array_Add` (`self.pcs`) NewPlayer))

(event `self.K2_OnLogout`
  (params (ExitingController :type "Controller Object Reference"))
  (cast `/Game/Blueprint/Lobby/LobbyPC` ExitingController))

(event `InitPlayer`
  (params (pc :type "PlayerController Object Reference"))
  (bind _idx (`self.FindPlayerSpawn`))
  (bind _actor (`self.SpawnActor` _idx pc))
  (`self.SetActorName` pc _actor)
  (`self.HideQuitParty_BTN` pc)
  (`self.HideSearch_BTN` pc))

(fn `FindPlayerSpawn`
  (returns (idx :type Integer))
  (bind _outactors (`GameplayStatics.GetAllActorsOfClass` "/Game/Blueprint/Lobby/LobbySpawn.LobbySpawn_C"))
  (if (== (`self.NumPlayers`) 1)
    (`/Game/Blueprint/Lobby/LobbySpawn.setSlotState` (`|GetArrayItem` _outactors) true)
    (return 0)
    (else
      (for (_array_element _array_index) _outactors
        (if (not (`/Game/Blueprint/Lobby/LobbySpawn.SlotUsed` _array_element))
          (`/Game/Blueprint/Lobby/LobbySpawn.setSlotState` _array_element true)
          (`self.Send Slot State`)
          (return _array_index))))))

(fn `HideQuitParty_BTN`
  (params (pc :type "PlayerController Object Reference"))
  (if (== (`self.NumPlayers`) 1)
    (bind _aslobby_pc (cast `/Game/Blueprint/Lobby/LobbyPC` pc))
    (`/Game/Blueprint/Lobby/LobbyPC.HideQuitPartyBTN` _aslobby_pc)))

(fn `HideSearch_BTN`
  (params (pc :type "PlayerController Object Reference"))
  (if (not (== (`self.NumPlayers`) 1))
    (bind _aslobby_pc (cast `/Game/Blueprint/Lobby/LobbyPC` pc))
    (`/Game/Blueprint/Lobby/LobbyPC.HideSearchBTN` _aslobby_pc)))

(fn `Send Slot State`
  (bind _outactors (`GameplayStatics.GetAllActorsOfClass` "/Game/Blueprint/Lobby/LobbySpawn.LobbySpawn_C"))
  (for _array_element (`self.pcs`)
    (bind _aslobby_pc (cast `/Game/Blueprint/Lobby/LobbyPC` _array_element))
    (for _array_element_2 _outactors
      (`/Game/Blueprint/Lobby/LobbyPC.SetUsedSlot` _aslobby_pc (`/Game/Blueprint/Lobby/LobbySpawn.SlotUsed` _array_element_2) _array_element_2))))

(fn `SetActorName`
  (params (pc :type "PlayerController Object Reference") (actor :type "/Game/Blueprint/Lobby/LobbyActor Object Reference"))
  (bind _aslobby_pc (cast `/Game/Blueprint/Lobby/LobbyPC` pc))
  (bind _output_get (set `/Game/Blueprint/Lobby/LobbyPC.nickname` (`PlayerState.GetPlayerName` (`Controller.PlayerState` _aslobby_pc)) _aslobby_pc))
  (`/Game/Blueprint/Lobby/LobbyActor.SetPlayerNameLocal` actor _output_get))

(fn `SpawnActor`
  (params (idx :type Integer) (pc :type "PlayerController Object Reference"))
  (returns (actor :type "/Game/Blueprint/Lobby/LobbyActor Object Reference"))
  (bind _outactors (`GameplayStatics.GetAllActorsOfClass` "/Game/Blueprint/Lobby/LobbySpawn.LobbySpawn_C"))
  (bind _output (`|GetArrayItem` _outactors idx))
  (bind _returnvalue (`|SpawnActorFromClass` "/Game/Blueprint/Lobby/LobbyActor.LobbyActor_C" (`KismetMathLibrary.MakeTransform` (`self.K2_GetActorLocation` _output)) "AlwaysSpawn" "OverrideRootScale" null null))
  (bind _aslobby_pc (cast `/Game/Blueprint/Lobby/LobbyPC` pc))
  (set `/Game/Blueprint/Lobby/LobbyPC.LobbyActor` _returnvalue _aslobby_pc)
  (bind _output_get (set `/Game/Blueprint/Lobby/LobbyPC.Lobby Spawn` _output _aslobby_pc))
  (`/Game/Blueprint/Lobby/LobbyPC.client_lobbySpawn` _aslobby_pc _output_get)
  (return _returnvalue))

(fn `UpdatePlayerName`
  (for _array_element (`self.pcs`)
    (bind _aslobby_pc (cast `/Game/Blueprint/Lobby/LobbyPC` _array_element))
    (bind _lobbyactor (`/Game/Blueprint/Lobby/LobbyPC.LobbyActor` _aslobby_pc))
    (`/Engine/EditorBlueprintResources/StandardMacros.IsValid` _lobbyactor
      (:`Is Valid`
        (`/Game/Blueprint/Lobby/LobbyActor.SetPlayerNameLocal` _lobbyactor (`PlayerState.GetPlayerName` (`Controller.PlayerState` _array_element)))))))

(fn `UserConstructionScript`)