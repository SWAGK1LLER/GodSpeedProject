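; Main menu player controller that sets up the menu UI and the player's lobby character.
; On local BeginPlay it loads save data through EOSGameInstance, creates the main and lobby widgets, then asks MainMenuGameMode to spawn the saved default Thief or Officer.
; Events swap the two menus, forward team and name updates, and hide lobby buttons.
; Disconnecting frees the lobby slot via server and multicast-named events and destroys the lobby actor.
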(event `SpawnActor`
  (params (pc :type "PlayerController Object Reference") (character :type "EDefaultCharacter Enum" :default "Thief"))
  (bind _asmain_menu_game_mode (cast `/Game/Blueprint/MainMenu/MainMenuGameMode` (`GameplayStatics.GetGameMode`)))
  (`/Game/Blueprint/MainMenu/MainMenuGameMode.InitPlayer` _asmain_menu_game_mode pc character))

(event `self.ReceiveBeginPlay`
  (bind _returnvalue (`GameplayStatics.GetPlayerController` 0))
  (if (`self.IsLocalPlayerController`)
    (`|ExecutionSequence`
      (:`then_0`
        (bind _aseosgame_instance (cast `EOSGameInstance` (`GameplayStatics.GetGameInstance`)))
        (`EOSGameInstance.LoadSaveGame` _aseosgame_instance)
        (`EOSGameInstance.LoadSaveSettings` _aseosgame_instance))
      (:`then_1`
        (bind _returnvalue_2 (`|GenericCreateObject` "/Game/Blueprint/Widgets/BP_MainMenuButton.BP_MainMenuButton_C"))
        (bind _output_get (set `self.menuButtonWidget` _returnvalue_2))
        (`UserWidget.AddToViewport` _output_get 0)
        (set `PlayerController.bShowMouseCursor` true _returnvalue)
        (set `PlayerController.bEnableMouseOverEvents` true _returnvalue))
      (:`then_2`
        (bind _returnvalue_3 (`|GenericCreateObject` "/Game/Blueprint/MainMenu/LobbyMenu.LobbyMenu_C"))
        (`UserWidget.AddToViewport` _returnvalue_3 0)
        (bind _output_get_2 (set `self.LobbyMenu` _returnvalue_3))
        (`Widget.RemoveFromParent` _output_get_2)
        (set `/Game/Blueprint/MainMenu/LobbyMenu.pc` self _output_get_2)
        (bind _aseosgame_instance_2 (cast `EOSGameInstance` (`GameplayStatics.GetGameInstance`)))
        (bind _returnvalue_4 (`EOSGameInstance.GetPlayerSaveGame` _aseosgame_instance_2))
        (switch `int` (`PlayerSaveGame.defaultCharacter` _returnvalue_4)
          (:`0`
            (`self.SpawnActor` self)
            (`self.UpdatePlayerName`))
          (:`1`
            (`self.SpawnActor` self "Officer")
            (`self.UpdatePlayerName`)))))))

(event `UpdatePlayerName`
  (bind _asmain_menu_game_mode (cast `/Game/Blueprint/MainMenu/MainMenuGameMode` (`GameplayStatics.GetGameMode`)))
  (`/Game/Blueprint/MainMenu/MainMenuGameMode.UpdatePlayerName` _asmain_menu_game_mode))

(event `SetTeam`
  (params (team :type "ETeam Enum" :default "A"))
  (bind _aseosgame_instance (cast `EOSGameInstance` (`GameplayStatics.GetGameInstance`)))
  (set `EOSGameInstance.team` team _aseosgame_instance))

(event `HideQuitPartyBTN`
  (`/Game/Blueprint/MainMenu/LobbyMenu.HideQuitBTN` (`self.LobbyMenu`)))

(event `HideSearchBTN`
  (`/Game/Blueprint/MainMenu/LobbyMenu.HideSearchBTN` (`self.LobbyMenu`)))

(event `TurnOffOutLine`
  (`/Game/Blueprint/MainMenu/MainMenuOfficer.turnOffOutline` (`self.secuActor`))
  (`/Game/Blueprint/MainMenu/MainMenuThief.turnOffOutline` (`self.secuThief`)))

(event `DestroyPlayer`
  (`self.SR_DisconnectPlayer` (`self.Lobby Spawn`))
  (`self.K2_DestroyActor` (`self.LobbyActor`)))

(event `SetUsedSlot`
  (params (used :type Boolean) (playerStart :type "/Game/Blueprint/MainMenu/LobbySpawn Object Reference"))
  (`/Game/Blueprint/MainMenu/LobbySpawn.setSlotState` playerStart used))

(event `ShowMainMenu`
  (`UserWidget.AddToViewport` (`self.menuButtonWidget`) 0)
  (`Widget.RemoveFromParent` (`self.LobbyMenu`)))

(event `client_lobbySpawn`
  (params (spawn :type "/Game/Blueprint/MainMenu/LobbySpawn Object Reference (by ref)"))
  (set `self.Lobby Spawn` spawn))

(event `ShowGameMenu`
  (`UserWidget.AddToViewport` (`self.LobbyMenu`) 0)
  (`Widget.RemoveFromParent` (`self.menuButtonWidget`)))

(event `SR_DisconnectPlayer`
  (params (spawn :type "/Game/Blueprint/MainMenu/LobbySpawn Object Reference"))
  (`self.multi_createInviteUI` spawn))

(event `multi_createInviteUI`
  (params (lobby :type "/Game/Blueprint/MainMenu/LobbySpawn Object Reference"))
  (`/Game/Blueprint/MainMenu/LobbySpawn.setSlotState` lobby false))

(fn `Disconnect`
  (`self.SetUsedSlot` false (`self.Lobby Spawn`))
  (`self.DestroyPlayer`))

(fn `UserConstructionScript`)