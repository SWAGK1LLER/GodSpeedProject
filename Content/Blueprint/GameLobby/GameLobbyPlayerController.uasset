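; Player controller for the game lobby that registers the player's team and handles team switching and debug launch.
; On BeginPlay, the local controller reads its team from EOSGameInstance and has GameLobbyGameMode count it, initialize the player and update names.
; T flips the stored team between Thief (A) and Security (B) without re-registering.
; Outside distribution builds, it shows a debug widget and L force-launches the game.
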(event `printLocal`
  (params (string :type String))
  (`self.printLocal` string))

(event `Key|T`
  (params (Key :type "Key Structure"))
  (:`Pressed`
    (bind _aseosgame_instance (cast `EOSGameInstance` (`GameplayStatics.GetGameInstance`)))
    (switch `ETeam` (`EOSGameInstance.team` _aseosgame_instance)
      (:`A`
        (set `EOSGameInstance.team` "B" _aseosgame_instance)
        (`self.printLocal` "Your now team Security"))
      (:`B`
        (set `EOSGameInstance.team` "A" _aseosgame_instance)
        (`self.printLocal` "Your now team Thief")))))

(event `ForceLaunchGame`
  (bind _asgame_lobby_game_mode (cast `/Game/Blueprint/GameLobby/GameLobbyGameMode` (`GameplayStatics.GetGameMode`)))
  (`/Game/Blueprint/GameLobby/GameLobbyGameMode.ForceLaunch` _asgame_lobby_game_mode))

(event `Key|L`
  (params (Key :type "Key Structure"))
  (:`Pressed`
    (if (not (`KismetSystemLibrary.IsPackagedForDistribution`))
      (`self.ForceLaunchGame`))))

(event `AddDebugMessage`
  (if (not (`KismetSystemLibrary.IsPackagedForDistribution`))
    (bind _returnvalue (`|GenericCreateObject` "/Game/Blueprint/GameLobby/bp_debugMessage.bp_debugMessage_C"))
    (`UserWidget.AddToViewport` _returnvalue 0)))

(event `self.ReceiveBeginPlay`
  (`self.AddDebugMessage`)
  (if (`self.IsLocalController`)
    (`|ExecutionSequence`
      (:`then_0`
        (bind _aseosgame_instance (cast `EOSGameInstance` (`GameplayStatics.GetGameInstance`)))
        (`self.SetTeam` (`EOSGameInstance.team` _aseosgame_instance)))
      (:`then_1`
        (bind _aseosgame_instance_2 (cast `EOSGameInstance` (`GameplayStatics.GetGameInstance`)))
        (switch `ETeam` (`EOSGameInstance.team` _aseosgame_instance_2)
          (:`A`
            (`self.SpawnActor` self "TeamA"))
          (:`B`
            (`self.SpawnActor` null "TeamB")))
        (`self.UpdatePlayerName`)))))

(event `SetTeam`
  (params (team :type "ETeam Enum" :default "A"))
  (switch `ETeam` team
    (:`A`
      (bind _asgame_lobby_game_mode (cast `/Game/Blueprint/GameLobby/GameLobbyGameMode` (`GameplayStatics.GetGameMode`)))
      (`/Game/Blueprint/GameLobby/GameLobbyGameMode.AddToTeamA` _asgame_lobby_game_mode))
    (:`B`
      (bind _asgame_lobby_game_mode_2 (cast `/Game/Blueprint/GameLobby/GameLobbyGameMode` (`GameplayStatics.GetGameMode`)))
      (`/Game/Blueprint/GameLobby/GameLobbyGameMode.AddToTeamB` _asgame_lobby_game_mode_2))))

(event `SpawnActor`
  (params (pc :type "PlayerController Object Reference") (teamString :type String))
  (bind _asgame_lobby_game_mode (cast `/Game/Blueprint/GameLobby/GameLobbyGameMode` (`GameplayStatics.GetGameMode`)))
  (`/Game/Blueprint/GameLobby/GameLobbyGameMode.InitPlayer` _asgame_lobby_game_mode pc teamString))

(event `UpdatePlayerName`
  (bind _asgame_lobby_game_mode (cast `/Game/Blueprint/GameLobby/GameLobbyGameMode` (`GameplayStatics.GetGameMode`)))
  (`/Game/Blueprint/GameLobby/GameLobbyGameMode.Update Player Name` _asgame_lobby_game_mode))

(fn `UserConstructionScript`)