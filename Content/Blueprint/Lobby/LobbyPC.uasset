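; LobbyPC is the lobby player controller that links each player's menu and lobby actor to the game mode.
; On BeginPlay, the local controller creates the LobbyMenu widget, then asks LobbyGameMode to initialize the player and update player names.
; Other events store the team in EOSGameInstance and hide the menu's quit-party and search buttons.
; Disconnect tells the lobby actor to disconnect, then destroys it.
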(event `self.ReceiveBeginPlay`
  (if (`self.IsLocalPlayerController`)
    (bind _returnvalue (`|GenericCreateObject` "/Game/Blueprint/Lobby/LobbyMenu.LobbyMenu_C"))
    (bind _output_get (set `self.LobbyMenu` _returnvalue))
    (`UserWidget.AddToViewport` _output_get 0)
    (`self.SpawnActor` self)
    (`self.UpdatePlayerName`)))

(event `SpawnActor`
  (params (pc :type "PlayerController Object Reference"))
  (bind _aslobby_game_mode (cast `/Game/Blueprint/Lobby/LobbyGameMode` (`GameplayStatics.GetGameMode`)))
  (`/Game/Blueprint/Lobby/LobbyGameMode.InitPlayer` _aslobby_game_mode pc))

(event `UpdatePlayerName`
  (bind _aslobby_game_mode (cast `/Game/Blueprint/Lobby/LobbyGameMode` (`GameplayStatics.GetGameMode`)))
  (`/Game/Blueprint/Lobby/LobbyGameMode.UpdatePlayerName` _aslobby_game_mode))

(event `SetTeam`
  (params (team :type "ETeam Enum" :default "A"))
  (bind _aseosgame_instance (cast `EOSGameInstance` (`GameplayStatics.GetGameInstance`)))
  (set `EOSGameInstance.team` team _aseosgame_instance))

(event `HideQuitPartyBTN`
  (`/Game/Blueprint/Lobby/LobbyMenu.HideQuitBTN` (`self.LobbyMenu`)))

(event `HideSearchBTN`
  (`/Game/Blueprint/Lobby/LobbyMenu.HideSearchBTN` (`self.LobbyMenu`)))

(event `DestroyPlayer`
  (`self.K2_DestroyActor` (`self.LobbyActor`)))

(fn `Disconnect`
  (`/Game/Blueprint/Lobby/LobbyActor.Disconnect` (`self.LobbyActor`))
  (`self.DestroyPlayer`))

(fn `UserConstructionScript`)