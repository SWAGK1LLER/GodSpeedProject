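; GameInstance Blueprint that relays online login, party and game search results and routes team selection in the lobby.
; Its login, party-join failure and search events each fire a matching Call, passing the message along for a failed party join.
; SetPlayerTeam casts the current game mode to LobbyGameMode and forwards the chosen team to it, doing nothing when the cast fails.
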(event `self.LoginSuccessful`
  (`self.LoginSuccess`))

(event `self.LoginFail`
  (`self.LoginFailed`))

(event `self.JoinPartyFail`
  (params (msg :type String))
  (`self.JoinPartyFailed` msg))

(event `self.SearchFail`
  (`self.SearchGameFailed`))

(event `self.SearchFinish`
  (`self.SearchGameFinished`))

(event `self.setPlayerTeam`
  (params (aTeam :type "ETeam Enum" :default "A"))
  (bind _aslobby_game_mode (cast `/Game/Blueprint/Lobby/LobbyGameMode` (`GameplayStatics.GetGameMode`)))
  (`/Game/Blueprint/Lobby/LobbyGameMode.SetTeam` _aslobby_game_mode aTeam))