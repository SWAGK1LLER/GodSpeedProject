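; Game mode for a two-team match that spawns players as thieves (Team A) or officers (Team B).
; SpawnPlayer records the controller in its team array, destroys any existing pawn, then spawns and possesses the team's Base3C character.
; FindPlayerSpawn claims the first unused GamePlayerStart tagged for that team, and GetTeamMate returns a team's list.
; BeginPlay only casts the EOS game instance; its StartGame call is disconnected.
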(event `self.ReceiveBeginPlay`
  (bind _aseosgame_instance (cast `EOSGameInstance` (`GameplayStatics.GetGameInstance`))))

(fn `FindPlayerSpawn`
  (params (TeamSide :type "ETeam Enum" :default "A"))
  (returns (Location :type "Transform Structure") (actor :type "Actor Class Reference"))
  (switch `ETeam` TeamSide
    (:`A`
      (bind _outactors (`GameplayStatics.GetAllActorsOfClassWithTag` "/Game/Blueprint/Game/GamePlayerStart.GamePlayerStart_C" "TeamA"))
      (for _array_element _outactors
        (bind _asgame_player_start (cast `/Game/Blueprint/Game/GamePlayerStart` _array_element))
        (if (not (`/Game/Blueprint/Game/GamePlayerStart.used` _asgame_player_start))
          (set `/Game/Blueprint/Game/GamePlayerStart.used` true _asgame_player_start)
          (return (`KismetMathLibrary.Conv_VectorToTransform` (`self.K2_GetActorLocation` _asgame_player_start)) "/Game/Blueprint/Game/Character/BP_Thief.BP_Thief_C"))))
    (:`B`
      (bind _outactors_2 (`GameplayStatics.GetAllActorsOfClassWithTag` "/Game/Blueprint/Game/GamePlayerStart.GamePlayerStart_C" "TeamB"))
      (for _array_element_2 _outactors_2
        (bind _asgame_player_start_2 (cast `/Game/Blueprint/Game/GamePlayerStart` _array_element_2))
        (if (not (`/Game/Blueprint/Game/GamePlayerStart.used` _asgame_player_start_2))
          (set `/Game/Blueprint/Game/GamePlayerStart.used` true _asgame_player_start_2)
          (return (`KismetMathLibrary.Conv_VectorToTransform` (`self.K2_GetActorLocation` _asgame_player_start_2)) "/Game/Blueprint/Game/Character/BP_Officer.BP_Officer_C"))))))

(fn `GetTeamMate`
  (params (TeamSide :type "ETeam Enum" :default "A"))
  (returns (TeamMate :type "Array of PlayerController Object Reference"))
  (switch `ETeam` TeamSide
    (:`A`
      (return (`self.TeamA`)))
    (:`B`
      (return (`self.TeamB`)))))

(fn `SpawnPlayer`
  (params (TeamSide :type "ETeam Enum" :default "A") (PC :type "PlayerController Object Reference"))
  (returns (pawn :type "Character Object Reference"))
  (bind _returnvalue (`Controller.K2_GetPawn` PC))
  (switch `ETeam` TeamSide
    (:`A`
      (`KismetArrayLibrary.Array_Add` (`self.TeamA`) PC))
    (:`B`
      (`KismetArrayLibrary.Array_Add` (`self.TeamB`) PC)))
  (`/Engine/EditorBlueprintResources/StandardMacros.IsValid` _returnvalue
    (:`Is Valid`
      (`self.K2_DestroyActor` _returnvalue))
    (:`Is Not Valid`
      _))
  (bind (_location _actor) (`self.FindPlayerSpawn` TeamSide))
  (bind _returnvalue_2 (`|SpawnActorFromClass` _actor _location "Undefined" "OverrideRootScale" null null))
  (bind _asbase_3c (cast `Base3C` _returnvalue_2))
  (`Controller.Possess` PC _asbase_3c)
  (return _asbase_3c))

(fn `UserConstructionScript`)