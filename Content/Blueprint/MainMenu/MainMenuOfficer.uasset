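; Main menu officer actor that acts as a clickable character for opening security customization.
; On BeginPlay it registers itself as SecuActor on BP_mainMenuPC.
; Hovering toggles a custom-depth outline on the skeletal mesh.
; Clicking has the controller clear outlines, shows the security customization menu through its button widget, and keeps this outline on until turnOffOutline resets it.
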(event `clickedOnActor`
  (bind _asbp_main_menu_pc (cast `/Game/Blueprint/MainMenu/BP_mainMenuPC` (`GameplayStatics.GetPlayerController` 0)))
  (`/Game/Blueprint/MainMenu/BP_mainMenuPC.TurnOffOutLine` _asbp_main_menu_pc)
  (`/Game/Blueprint/Widgets/BP_MainMenuButton.ShowCustomizationSecu` (`/Game/Blueprint/MainMenu/BP_mainMenuPC.menuButtonWidget` _asbp_main_menu_pc))
  (set `self.clicked` true)
  (`PrimitiveComponent.SetRenderCustomDepth` (`self.SkeletalMesh`) true))

(event `self.SkeletalMesh.OnClicked`
  (params (TouchedComponent :type "PrimitiveComponent Object Reference") (ButtonPressed :type "Key Structure"))
  (`self.clickedOnActor`))

(event `self.ReceiveActorBeginCursorOver`
  (`PrimitiveComponent.SetRenderCustomDepth` (`self.SkeletalMesh`) true))

(event `self.ReceiveActorEndCursorOver`
  (if (not (`self.clicked`))
    (`PrimitiveComponent.SetRenderCustomDepth` (`self.SkeletalMesh`) false)))

(event `turnOffOutline`
  (set `self.clicked` false)
  (`PrimitiveComponent.SetRenderCustomDepth` (`self.SkeletalMesh`) false))

(event `self.ReceiveBeginPlay`
  (bind _asbp_main_menu_pc (cast `/Game/Blueprint/MainMenu/BP_mainMenuPC` (`GameplayStatics.GetPlayerController` 0)))
  (set `/Game/Blueprint/MainMenu/BP_mainMenuPC.secuActor` self _asbp_main_menu_pc))

(fn `UserConstructionScript`)