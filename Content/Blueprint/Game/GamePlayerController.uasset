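; Player controller that requests a team-based spawn for its player when a match level starts.
; On BeginPlay, the local controller reads Team from the EOSGameInstance and passes it to the SR_SpawnPlayer event.
; That event casts to GameGameMode and calls SpawnPlayer with the team and itself, leaving the spawn to the game mode.
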(event `self.ReceiveBeginPlay`
  (if (`self.IsLocalPlayerController`)
    (bind _aseosgame_instance (cast `EOSGameInstance` (`GameplayStatics.GetGameInstance`)))
    (`self.SR_SpawnPlayer` (`EOSGameInstance.team` _aseosgame_instance))))

(event `SR_SpawnPlayer`
  (params (TeamSide :type "ETeam Enum" :default "A"))
  (bind _asgame_game_mode (cast `/Game/Blueprint/Game/GameGameMode` (`GameplayStatics.GetGameMode`)))
  (`/Game/Blueprint/Game/GameGameMode.SpawnPlayer` _asgame_game_mode TeamSide self))

(fn `UserConstructionScript`)