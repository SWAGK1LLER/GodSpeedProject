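; Player controller that requests a team-based spawn and owns the inventory HUD for a Thief pawn.
; On local BeginPlay it passes the team stored in EOSGameInstance to SR_SpawnPlayer, which has GameGameMode spawn the player.
; Possessing a Thief creates local Inventory and TeamInventory widgets, with an event refreshing the personal one.
; The team inventory refresh is unfinished: it only casts a TeamA member's pawn, leaving bag updates unconnected.
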(event `self.ReceiveBeginPlay`
  (if (`self.IsLocalPlayerController`)
    (bind _aseosgame_instance (cast `EOSGameInstance` (`GameplayStatics.GetGameInstance`)))
    (`self.SR_SpawnPlayer` (`EOSGameInstance.team` _aseosgame_instance))))

(event `SR_SpawnPlayer`
  (params (TeamSide :type "ETeam Enum" :default "A"))
  (bind _asgame_game_mode (cast `/Game/Blueprint/Game/GameGameMode` (`GameplayStatics.GetGameMode`)))
  (`/Game/Blueprint/Game/GameGameMode.SpawnPlayer` _asgame_game_mode TeamSide self))

(event `self.PawnIsPossess`
  (params (InPawn :type "Pawn Object Reference"))
  (if (`self.IsLocalPlayerController`)
    (bind _asthief (cast `Thief` InPawn))
    (`|ExecutionSequence`
      (:`then_0`
        (bind _returnvalue (`|GenericCreateObject` _asthief "/Game/Blueprint/Game/Inventory/Inventory.Inventory_C"))
        (bind _output_get (set `self.InventoryWidget` _returnvalue))
        (`UserWidget.AddToViewport` _output_get 0))
      (:`then_1`
        (bind _returnvalue_2 (`|GenericCreateObject` _asthief "/Game/Blueprint/Game/Inventory/TeamInventory.TeamInventory_C"))
        (bind _output_get_2 (set `self.TeamInventoryWidget` _returnvalue_2))
        (`UserWidget.AddToViewport` _output_get_2 0)))))

(event `self.UpdateInventoryUI`
  (params (pItems :type "Array of ItemLooted Structure (by ref)"))
  (if (`self.IsLocalPlayerController`)
    (`/Game/Blueprint/Game/Inventory/Inventory.UpdateInventory` (`self.InventoryWidget`) pItems)))

(event `UpdateTeamInventoryUI`
  (bind _asgame_game_mode (cast `/Game/Blueprint/Game/GameGameMode` (`GameplayStatics.GetGameMode`)))
  (`|ExecutionSequence`
    (:`then_1`
      (bind _asthief (cast `Thief` (`self.K2_GetPawn` (`|GetArrayItem` (`/Game/Blueprint/Game/GameGameMode.TeamA` _asgame_game_mode) 1)))))))

(fn `UserConstructionScript`)