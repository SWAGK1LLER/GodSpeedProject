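; Game mode for the pre-match lobby that registers players with the EOS session and server-travels to the LevelDesign map at six players or on a forced launch.
; Team join events increment TeamA/TeamB counts and push them to the game instance's session settings.
; InitPlayer claims a free team-tagged GameLobbySpawn, spawns a Thief (TeamA) or Officer lobby actor there, and labels it with the player's name.
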(event `ForceLaunch`
  (`KismetSystemLibrary.ExecuteConsoleCommand` "ServerTravel /Game/Maps/LevelDesign?listen" null))

(event `self.K2_PostLogin`
  (params (NewPlayer :type "PlayerController Object Reference"))
  (bind _pcs (`self.pcs`))
  (bind _returnvalue (`KismetArrayLibrary.Array_Add` _pcs NewPlayer))
  (bind _aseosgame_instance (cast `EOSGameInstance` (`GameplayStatics.GetGameInstance`)))
  (`EOSGameInstance.registerPlayerToGameSession` _aseosgame_instance NewPlayer)
  (set `EOSGameInstance.TotalConnectedPlayer` (+ _returnvalue 1) _aseosgame_instance)
  (if (== (`KismetArrayLibrary.Array_Length` _pcs) 6)
    (`KismetSystemLibrary.ExecuteConsoleCommand` "ServerTravel /Game/Maps/LevelDesign?listen" null)))

(event `self.K2_OnLogout`
  (params (ExitingController :type "Controller Object Reference"))
  (bind _aseosgame_instance (cast `EOSGameInstance` (`GameplayStatics.GetGameInstance`)))
  (bind _asplayer_controller (cast `PlayerController` ExitingController))
  (`EOSGameInstance.unregisterPlayerToGameSession` _aseosgame_instance _asplayer_controller))

(event `AddToTeamB`
  (bind _result (`/Engine/EditorBlueprintResources/StandardMacros.IncrementInt` (`self.TeamB`))
    (:`  `
      (bind _aseosgame_instance (cast `EOSGameInstance` (`GameplayStatics.GetGameInstance`) :!label _label))
      (`EOSGameInstance.updateGameSettings` _aseosgame_instance (stale `AddToTeamA` _result) _result))))

(event `AddToTeamA`
  (bind _result (`/Engine/EditorBlueprintResources/StandardMacros.IncrementInt` (`self.TeamA`))
    (:`  `
      (goto _label))))

(event `InitPlayer`
  (params (pc :type "PlayerController Object Reference") (teamSide :type String))
  (bind _idx (`self.FindPlayerSpawn` teamSide))
  (bind _actor (`self.SpawnActor` _idx pc teamSide))
  (`self.SetActorName` pc _actor))

(fn `FindPlayerSpawn`
  (params (teamSide :type String))
  (returns (idx :type Integer))
  (bind _outactors (`GameplayStatics.GetAllActorsOfClassWithTag` "/Game/Blueprint/GameLobby/GameLobbySpawn.GameLobbySpawn_C" (`KismetStringLibrary.Conv_StringToName` teamSide)))
  (if (== (`self.NumPlayers`) 1)
    (`/Game/Blueprint/GameLobby/GameLobbySpawn.setSlotState` (`|GetArrayItem` _outactors) true)
    (return 0)
    (else
      (for (_array_element _array_index) _outactors
        (if (not (`/Game/Blueprint/GameLobby/GameLobbySpawn.SlotUsed` _array_element))
          (`/Game/Blueprint/GameLobby/GameLobbySpawn.setSlotState` _array_element true)
          (return _array_index))))))

(fn `SetActorName`
  (params (pc :type "PlayerController Object Reference") (actor :type "/Game/Blueprint/GameLobby/GameLobbyActor Object Reference"))
  (locals (NewLocalVar :type "/Game/Blueprint/MainMenu/LobbyActor Object Reference"))
  (bind _asgame_lobby_player_controller (cast `/Game/Blueprint/GameLobby/GameLobbyPlayerController` pc))
  (bind _output_get (set `/Game/Blueprint/GameLobby/GameLobbyPlayerController.nickname` (`PlayerState.GetPlayerName` (`Controller.PlayerState` _asgame_lobby_player_controller)) _asgame_lobby_player_controller))
  (`/Game/Blueprint/GameLobby/GameLobbyActor.SetPlayerNameLocal` actor _output_get))

(fn `SpawnActor`
  (params (idx :type Integer) (pc :type "PlayerController Object Reference") (TeamSide :type String))
  (returns (actor :type "/Game/Blueprint/GameLobby/GameLobbyActor Object Reference"))
  (bind _returnvalue (`KismetStringLibrary.Conv_StringToName` TeamSide))
  (bind _outactors (`GameplayStatics.GetAllActorsOfClassWithTag` "/Game/Blueprint/GameLobby/GameLobbySpawn.GameLobbySpawn_C" _returnvalue))
  (bind _output (`|GetArrayItem` _outactors idx))
  (bind _returnvalue_2 (`|SpawnActorFromClass` "/Game/Blueprint/GameLobby/GameLobbyActor.GameLobbyActor_C" (`KismetMathLibrary.MakeTransform` (`self.K2_GetActorLocation` _output)) "AlwaysSpawn" "OverrideRootScale" null null))
  (if (== _returnvalue "TeamA")
    (set `/Game/Blueprint/GameLobby/GameLobbyActor.mesh` "/Game/3D_Assets/Character/thief.thief" _returnvalue_2)
    (else
      (set `/Game/Blueprint/GameLobby/GameLobbyActor.mesh` "/Game/3D_Assets/Character/officer.officer" _returnvalue_2)))
  (bind _asgame_lobby_player_controller (cast `/Game/Blueprint/GameLobby/GameLobbyPlayerController` pc))
  (bind _output_get (set `/Game/Blueprint/GameLobby/GameLobbyPlayerController.lobbyActor` _returnvalue_2 _asgame_lobby_player_controller))
  (set `/Game/Blueprint/GameLobby/GameLobbyActor.GameLobbySpawn` _output _output_get)
  (return _returnvalue_2))

(fn `Update Player Name`
  (for _array_element (`self.pcs`)
    (bind _asgame_lobby_player_controller (cast `/Game/Blueprint/GameLobby/GameLobbyPlayerController` _array_element))
    (bind _lobbyactor (`/Game/Blueprint/GameLobby/GameLobbyPlayerController.lobbyActor` _asgame_lobby_player_controller))
    (`/Engine/EditorBlueprintResources/StandardMacros.IsValid` _lobbyactor
      (:`Is Valid`
        (`/Game/Blueprint/GameLobby/GameLobbyActor.SetPlayerNameLocal` _lobbyactor (`PlayerState.GetPlayerName` (`Controller.PlayerState` _array_element)))))))

(fn `UserConstructionScript`)